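; HeadCollision is a Blueprint that pushes its Scene component back horizontally when its Sphere begins an overlap, apparently to keep the head out of geometry.
; Tick caches the Camera's world location in NewVar0.
; On overlap, it offsets Scene by the cached location minus the current one in X and Y, without sweep, undoing camera movement since that cache.
; The correction runs only on overlap begin, with no filtering of the overlapped object.
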(event OnComponentBeginOverlap(Sphere)
  (params (OverlappedComponent :type Primitive%20Component%20Object%20Reference) (OtherActor :type Actor%20Object%20Reference) (OtherComp :type Primitive%20Component%20Object%20Reference) (OtherBodyIndex :type Integer) (bFromSweep :type Boolean) (SweepResult :type Hit%20Result%20Structure%20%28by%20ref%29))
  (bind _newvar_0 (Variables|Default|GetNewVar_0))
  (bind _camera (Variables|Default|GetCamera))
  (bind _returnvalue (Transformation|GetWorldLocation _camera))
  (bind _returnvalue_2 (- _newvar_0 _returnvalue))
  (Transformation|AddWorldOffset (Variables|Default|GetScene) (Math|Vector|MakeVector (.x _returnvalue_2) (.y _returnvalue_2) 0.0) false false))

(event EventBeginPlay)

(event Collision|EventActorBeginOverlap
  (params (OtherActor :type Actor%20Object%20Reference)))

(event EventTick
  (params (DeltaSeconds :type Float%20%28single-precision%29))
  (Variables|Default|SetNewVar_0 (Transformation|GetWorldLocation (Variables|Default|GetCamera))))

(fn ConstructionScript)