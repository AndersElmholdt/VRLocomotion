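; VR walk-in-place locomotion pawn that reads both motion controllers as knee trackers, calibrated on input or shortly after BeginPlay.
; Knee Z-peak events derive step frequency, which with user height sets walking speed that decays over time since the last step.
; Tick moves VROffset along knee yaw and estimates body center to orient leg meshes.
; A Playback mode replaces controller input with recorded proxy transforms.
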(event OnPeakZ(RightPeakDetection)
  ;[1 1 1] Detect steps
  (CallFunction|Walk))

(event OnPeakZ(LeftPeakDetection)
  ;[1 1 1] Detect steps
  (CallFunction|Walk))

(event Custom|Walk
  ;[1 1 1] Start Walking
  (Variables|Default|SetStepFrequency (/ 1.0 (Math|Float|Absolute(Float) (- (.z (Class|PeakDetection|GetMinZ (Variables|Default|GetRight%20Peak%20Detection))) (.z (Class|PeakDetection|GetMinZ (Variables|Default|GetLeft%20Peak%20Detection)))))))
  (Variables|Default|SetWalkingspeed (CallFunction|KM/HtoM/S (Math|Float|Absolute(Float) (* (/ (Variables|Default|GetHeight) 1.72) (/ (Variables|Default|GetStepFrequency) 0.157))))))

(event Custom|PlaybackData
  (params (PlaybackOffset :type Boolean))
  (bind _rkp (Variables|Default|GetRKP))
  (bind _offsetp (Variables|Default|GetOffsetP))
  (bind _lkp (Variables|Default|GetLKP))
  (bind _offsetp_2 (Variables|Default|GetOffsetP))
  (bind _returnvalue (Transformation|GetWorldTransform _lkp))
  (bind _returnvalue_2 (Transformation|GetWorldTransform _offsetp_2))
  (bind _returnvalue_3 (Transformation|GetWorldTransform _rkp))
  (bind _returnvalue_4 (Transformation|GetWorldTransform _offsetp))
  (bind _outputtransform (CallFunction|MakeRelativeTransform _returnvalue _returnvalue_2))
  (bind _outputtransform_2 (CallFunction|MakeRelativeTransform _returnvalue_3 _returnvalue_4))
  ;[1 1 1] Playback Recording
  (if PlaybackOffset
    (Transformation|SetWorldTransform (Variables|Default|GetVR%20Offset) (Transformation|GetWorldTransform (Variables|Default|GetOffsetP)) false false))
  (Transformation|SetRelativeTransform (Variables|Default|GetRight%20Knee) (Math|Transform|MakeTransform (.location _outputtransform_2) (.rotation _outputtransform_2) "1.000000,1.000000,1.000000") false false)
  (Transformation|SetRelativeTransform (Variables|Default|GetLeft%20Knee) (Math|Transform|MakeTransform (.location _outputtransform) (.rotation _outputtransform) "1.000000,1.000000,1.000000") false false)
  (Transformation|SetRelativeTransform (Variables|Default|GetCamera) (CallFunction|MakeRelativeTransform (Transformation|GetWorldTransform (Variables|Default|GetCamP)) (Transformation|GetWorldTransform (Variables|Default|GetOffsetP))) false false))

(event Custom|Decay%20Speed
  ;[1 1 1] Decay Speed
  (Variables|Default|SetRealWalkingSpeed (Math|Float|Clamp(Float) (Math|Float|Lerp (Variables|Default|GetWalkingspeed) 0.0 (/ (- (Utilities|Time|GetTimeSeconds) (Math|Float|Max(Float) (.z (Class|PeakDetection|GetMinZ (Variables|Default|GetRight%20Peak%20Detection))) (.z (Class|PeakDetection|GetMinZ (Variables|Default|GetLeft%20Peak%20Detection))))) (Variables|Default|GetSpeedDecayTime))) 0.0 (Variables|Default|GetMaxSpeed))))

(event Custom|Calculate%20Body%20Center
  (bind _camera (Variables|Default|GetCamera))
  (bind _right_knee (Variables|Default|GetRight%20Knee))
  (bind _left_knee (Variables|Default|GetLeft%20Knee))
  (bind _right_knee_2 (Variables|Default|GetRight%20Knee))
  (bind _left_knee_2 (Variables|Default|GetLeft%20Knee))
  (bind _relativelocation (Variables|/Script/Engine.SceneComponent|GetRelativeLocation _camera))
  (bind _relativelocation_2 (Variables|/Script/Engine.SceneComponent|GetRelativeLocation _left_knee))
  (bind _relativelocation_3 (Variables|/Script/Engine.SceneComponent|GetRelativeLocation _right_knee))
  (bind _relativelocation_4 (Variables|/Script/Engine.SceneComponent|GetRelativeLocation _left_knee_2))
  (bind _relativelocation_5 (Variables|/Script/Engine.SceneComponent|GetRelativeLocation _right_knee_2))
  (bind _returnvalue (+ _relativelocation_3 _relativelocation_2))
  (bind _returnvalue_2 (/ _returnvalue 2.0))
  (bind _returnvalue_3 (- _relativelocation _returnvalue_2))
  (bind _returnvalue_4 (/ _returnvalue_3 2.0))
  (bind _returnvalue_5 (+ _returnvalue_4 _returnvalue_2))
  ;[1 1 1] Update Body Center
  (Transformation|SetRelativeLocation (Variables|Default|GetBodyCenter) (- (Math|Vector|MakeVector (.x _returnvalue_5) (.y _returnvalue_5) (+ (.Z (Math|Vector|BreakVector _returnvalue_2)) (Variables|Default|GetKneeHeight))) (* (Math|Vector|GetForwardVector (Variables|/Script/Engine.SceneComponent|GetRelativeRotation _left_knee)) 1e+01)) false false)
  (Transformation|SetRelativeTransform (Variables|Default|GetCylinder1) (Math|Transform|MakeTransform _relativelocation_4 (Class|QuaternionFunctions|ConverttoRotator (Class|QuaternionFunctions|CombineQuaternions (Class|QuaternionFunctions|ConverttoQuaternion (Math|Rotator|MakeRotfromZ (- (+ (Variables|/Script/Engine.SceneComponent|GetRelativeLocation (Variables|Default|GetBodyCenter)) "0, 0,50.000000") _relativelocation_4))) (Class|QuaternionFunctions|ConverttoQuaternion (Math|Rotator|MakeRotator 0.0 0.0 9e+01)))) "-1.000000,1.000000,1.000000") false false)
  (Transformation|SetRelativeTransform (Variables|Default|GetStaticMesh1) (Math|Transform|MakeTransform _relativelocation_5 (Class|QuaternionFunctions|ConverttoRotator (Class|QuaternionFunctions|CombineQuaternions (Class|QuaternionFunctions|ConverttoQuaternion (Math|Rotator|MakeRotfromZ (- (+ (Variables|/Script/Engine.SceneComponent|GetRelativeLocation (Variables|Default|GetBodyCenter)) "0,0.000000,50.000000") _relativelocation_5))) (Class|QuaternionFunctions|ConverttoQuaternion (Math|Rotator|MakeRotator 0.0 0.0 -9e+01)))) "1.000000,1.000000,1.000000") false false))

(event Custom|UpdatePosition
  (params (DeltaTime :type Float%20%28single-precision%29))
  (bind _left_knee (Variables|Default|GetLeft%20Knee))
  (bind _right_knee (Variables|Default|GetRight%20Knee))
  (bind _returnvalue (Transformation|GetWorldRotation _left_knee))
  (bind _returnvalue_2 (Transformation|GetWorldRotation _right_knee))
  ;[1 1 1] Update Position
  (Transformation|AddWorldOffset (Variables|Default|GetVR%20Offset) (* (* (Math|Vector|RotateVectorAroundAxis (Math|Vector|MakeVector (Variables|Default|GetRealWalkingSpeed) 0.0 0.0) (Math|Float|SelectFloat (/ (+ (.yaw _returnvalue) (.yaw _returnvalue_2)) 2.0) (.yaw _returnvalue) (== (Math|Float|Sign(Float) (.yaw _returnvalue)) (Math|Float|Sign(Float) (.yaw _returnvalue_2)))) "0, 0,1.000000") DeltaTime) (Variables|Default|GetSpeedMultiplier)) false false))

(event Custom|UpdateKnee
  (bind (_outposition _outorientation) (Class|SteamVRFunctionLibrary|GetHandPositionandOrientation 0 "Left"))
  (bind (_outposition_2 _outorientation_2) (Class|SteamVRFunctionLibrary|GetHandPositionandOrientation 0 "Right"))
  (bind _rightdeltarotation (Variables|Default|GetRightDeltaRotation))
  (bind _leftdeltarotation (Variables|Default|GetLeftDeltaRotation))
  ;[1 1 1] Update Knee Transform
  (Transformation|SetRelativeTransform (Variables|Default|GetRight%20Knee) (Math|Transform|MakeTransform _outposition_2 (Math|Rotator|CombineRotators "0,90.000000, 0" (Class|QuaternionFunctions|ConverttoRotator (Class|QuaternionFunctions|CombineQuaternions (Class|QuaternionFunctions|ConverttoQuaternion _outorientation_2) (Utilities|Struct|MakeQuat (.x _rightdeltarotation) (.y _rightdeltarotation) (.z _rightdeltarotation) (.w _rightdeltarotation))))) "0.100000,0.100000,0.100000") false false)
  (Transformation|SetRelativeTransform (Variables|Default|GetLeft%20Knee) (Math|Transform|MakeTransform _outposition (Math|Rotator|CombineRotators "0,90.000000, 0" (Class|QuaternionFunctions|ConverttoRotator (Class|QuaternionFunctions|CombineQuaternions (Class|QuaternionFunctions|ConverttoQuaternion _outorientation) (Utilities|Struct|MakeQuat (.x _leftdeltarotation) (.y _leftdeltarotation) (.z _leftdeltarotation) (.w _leftdeltarotation))))) "0.100000,0.100000,0.100000") false false))

(event EventBeginPlay
  (bind _outorientation (Class|SteamVRFunctionLibrary|GetHandPositionandOrientation 0 "Left"))
  (bind _right_knee (Variables|Default|GetRight%20Knee))
  (bind _returnvalue (Class|QuaternionFunctions|ConverttoQuaternion _outorientation))
  (bind _relativerotation (Variables|/Script/Engine.SceneComponent|GetRelativeRotation _right_knee))
  (bind _returnvalue_2 (Class|QuaternionFunctions|ConverttoQuaternion _relativerotation))
  (bind _returnvalue_3 (Class|QuaternionFunctions|InvertQuaternion _returnvalue))
  (bind _returnvalue_4 (Class|QuaternionFunctions|InvertQuaternion _returnvalue_2))
  ;[1 1 1] Initial Values
  (Utilities|FlowControl|Delay 1.0)
  (bind _output_get (Variables|Default|SetKneeHeight (.z (Variables|/Script/Engine.SceneComponent|GetRelativeLocation _right_knee))))
  (Transformation|SetRelativeLocation (Variables|Default|GetRight%20Foot) (Math|Vector|MakeVector 0.0 0.0 (* _output_get -1.0)) false false)
  (Transformation|SetRelativeLocation (Variables|Default|GetLeft%20Foot) (Math|Vector|MakeVector 0.0 0.0 (* _output_get -1.0)) false false)
  (Variables|Default|SetRightDeltaRotation (Utilities|Struct|MakeQuaternion (.x _returnvalue_4) (.y _returnvalue_4) (.z _returnvalue_4) (.w _returnvalue_4)))
  (Variables|Default|SetLeftDeltaRotation (Utilities|Struct|MakeQuaternion (.x _returnvalue_3) (.y _returnvalue_3) (.z _returnvalue_3) (.w _returnvalue_3)))
  (Variables|Default|SetHeight (/ (.z (Variables|/Script/Engine.SceneComponent|GetRelativeLocation (Variables|Default|GetCamera))) 1e+02))
  (Transformation|SetRelativeLocation (Variables|Default|GetBodyCenter) (+ (/ (+ (Variables|/Script/Engine.SceneComponent|GetRelativeLocation (Variables|Default|GetRight%20Knee)) (Variables|/Script/Engine.SceneComponent|GetRelativeLocation (Variables|Default|GetLeft%20Knee))) 2.0) (Math|Vector|MakeVector 0.0 0.0 (* (Variables|Default|GetKneeHeight) 1.0))) false false))

(event EventTick
  (params (DeltaSeconds :type Float%20%28single-precision%29))
  ;[1 1 1] Tick
  (if (Variables|Default|GetPlayback)
    (CallFunction|PlaybackData false)
    (CallFunction|UpdatePosition DeltaSeconds :!label _label)
    (CallFunction|DecaySpeed)
    (CallFunction|CalculateBodyCenter)
    (elif (CallFunction|ValidateMotionControllers)
      (CallFunction|UpdateKnee)
      (goto _label)
      (else
        (Development|PrintString "ERROR" true true "(R=1.000000,G=0.000000,B=0.000000,A=1.000000)")))))

(event Input|ActionEvents|InputActionCalibrate
  (params (Key :type Key%20Structure :default "AnyKey"))
  (bind _outorientation (Class|SteamVRFunctionLibrary|GetHandPositionandOrientation 0 "Left"))
  (bind _right_knee (Variables|Default|GetRight%20Knee))
  (bind _returnvalue (Class|QuaternionFunctions|ConverttoQuaternion _outorientation))
  (bind _relativerotation (Variables|/Script/Engine.SceneComponent|GetRelativeRotation _right_knee))
  (bind _returnvalue_2 (Class|QuaternionFunctions|ConverttoQuaternion _relativerotation))
  (bind _returnvalue_3 (Class|QuaternionFunctions|InvertQuaternion _returnvalue))
  (bind _returnvalue_4 (Class|QuaternionFunctions|InvertQuaternion _returnvalue_2))
  ;[1 1 1] Initial Values
  (:Pressed
    (bind _output_get (Variables|Default|SetKneeHeight (.z (Variables|/Script/Engine.SceneComponent|GetRelativeLocation _right_knee))))
    (Transformation|SetRelativeLocation (Variables|Default|GetRight%20Foot) (Math|Vector|MakeVector 0.0 0.0 (* _output_get -1.0)) false false)
    (Transformation|SetRelativeLocation (Variables|Default|GetLeft%20Foot) (Math|Vector|MakeVector 0.0 0.0 (* _output_get -1.0)) false false)
    (Variables|Default|SetRightDeltaRotation (Utilities|Struct|MakeQuaternion (.x _returnvalue_4) (.y _returnvalue_4) (.z _returnvalue_4) (.w _returnvalue_4)))
    (Variables|Default|SetLeftDeltaRotation (Utilities|Struct|MakeQuaternion (.x _returnvalue_3) (.y _returnvalue_3) (.z _returnvalue_3) (.w _returnvalue_3)))
    (Variables|Default|SetHeight (/ (.z (Variables|/Script/Engine.SceneComponent|GetRelativeLocation (Variables|Default|GetCamera))) 1e+02))
    (Transformation|SetRelativeLocation (Variables|Default|GetBodyCenter) (+ (/ (+ (Variables|/Script/Engine.SceneComponent|GetRelativeLocation (Variables|Default|GetRight%20Knee)) (Variables|/Script/Engine.SceneComponent|GetRelativeLocation (Variables|Default|GetLeft%20Knee))) 2.0) (Math|Vector|MakeVector 0.0 0.0 (* (Variables|Default|GetKneeHeight) 1.0))) false false)))

(fn ConstructionScript)

(fn MakeRelativeTransform
  (params (InputTransform :type Transform) (ParentTransform :type Transform))
  (return (Math|Transform|MakeTransform (- (.location InputTransform) (.location ParentTransform)) (Math|Rotator|CombineRotators (.rotation InputTransform) (Class|KismetMathLibrary|NegateRotator (.rotation ParentTransform))) (* (.scale InputTransform) (.scale ParentTransform)))))

(fn ValidateMotionControllers
  (return (and (.ReturnValue (Class|SteamVRFunctionLibrary|GetHandPositionandOrientation 0 "Right")) (.ReturnValue (Class|SteamVRFunctionLibrary|GetHandPositionandOrientation 0 "Left")))))

(fn KM/HtoM/S
  (params (KM/H :type Float%20%28single-precision%29))
  (return (/ (* KM/H 1e+03) 3.6e+03)))