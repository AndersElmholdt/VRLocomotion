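; BP_instancing_Tiles is an actor that lays out a flat grid of tiles from a single hierarchical instanced static mesh component.
; The construction script runs nested loops over XCount and YCount, adding one instance per cell at a fixed 400-unit spacing, then prints a completion message.
; The event graph holds only disabled default events, so all the work happens at construction.
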(event EventBeginPlay)

(event Collision|EventActorBeginOverlap
  (params (OtherActor :type Actor%20Object%20Reference)))

(event EventTick
  (params (DeltaSeconds :type Float%20%28single-precision%29)))

(fn ConstructionScript
  (for _index (range 0 (Variables|Default|GetXCount))
    (for _index_2 (range 0 (Variables|Default|GetYCount))
      (Components|InstancedStaticMesh|AddInstance (Variables|Default|GetHierarchicalInstancedStaticMesh) (Math|Transform|MakeTransform (Math|Vector|MakeVector (* _index 4e+02) (* _index_2 4e+02) 0.0)))))
  (Development|PrintString "Done"))