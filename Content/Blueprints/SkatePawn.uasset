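; VR pawn for riding a hoverboard by leaning, using motion controllers as knee trackers calibrated on start or input.
; Space spawns a board that glides in; standing on it starts skating, with stance detection, and stepping off destroys it.
; Head offset from the knee midpoint drives acceleration, braking and turning, moving the VR origin and rotating it around the camera.
; Playback mode substitutes recorded proxy transforms for live tracking.
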(event Custom|StartSkate
  ;[1 1 1] Start Skate
  (CallFunction|ApplyGoofy)
  (Variables|Default|SetSkating true)
  (Variables|Default|SetSkateSpeed 0.0)
  (Components|MoveComponentTo (Variables|Default|GetVR%20Offset) (Math|Vector|MakeVector 0.0 0.0 (+ (Variables|Default|GetBoardSpawnHeight) 5.0)) "0, 0, 0" true true 0.5 false))

(event Custom|UpdateDirection
  (bind _vr_origin (Variables|Default|GetVR%20Origin))
  (bind _rightknee (Variables|Default|GetRightKnee))
  (bind _rightknee_2 (Variables|Default|GetRightKnee))
  (bind _rightknee_3 (Variables|Default|GetRightKnee))
  (bind _returnvalue (Transformation|GetWorldRotation _rightknee_2))
  (bind _returnvalue_2 (Transformation|GetWorldRotation _rightknee))
  (bind _returnvalue_3 (Transformation|GetWorldRotation _rightknee_3))
  (bind _returnvalue_4 (Transformation|GetRelativeTransform _vr_origin))
  (bind _returnvalue_5 (Math|Vector|GetForwardVector _returnvalue))
  (bind _returnvalue_6 (Math|Vector|GetForwardVector _returnvalue_2))
  (bind _returnvalue_7 (Math|Rotator|CombineRotators (.rotation _returnvalue_4) _returnvalue_3))
  (bind (_x _y) (Math|Vector|BreakVector _returnvalue_5))
  (bind (_x_2 _y_2) (Math|Vector|BreakVector _returnvalue_6))
  (bind _returnvalue_8 (Math|Vector|GetForwardVector _returnvalue_7))
  (bind (_x_3 _y_3) (Math|Vector|BreakVector _returnvalue_8))
  ;[1 1 1] Change Stance
  (Variables|Default|SetDirection (Math|Vector|Normalize (Math|Vector|MakeVector _x_2 _y_2 0.0)))
  (Variables|Default|SetRealDirection (Math|Vector|Normalize (Math|Vector|MakeVector _x _y 0.0)))
  (Variables|Default|SetSkateDirection (Math|Vector|Normalize (Math|Vector|MakeVector _x_3 _y_3 0.0))))

(event Custom|StopSkate
  (bind _skateboard (Variables|Default|GetSkateboard))
  ;[1 1 1] Stop Skate
  (Variables|Default|SetSkating false)
  (if (Utilities|IsValid _skateboard)
    (Actor|DestroyActor _skateboard)
    (Components|MoveComponentTo (Variables|Default|GetVR%20Offset) "0, 0, 0" "0, 0, 0" true true 0.5 false)))

(event Custom|PlaybackData
  (params (PlaybackOffset :type Boolean))
  (bind _offsetp (Variables|Default|GetOffsetP))
  (bind _lkp (Variables|Default|GetLKP))
  (bind _rkp (Variables|Default|GetRKP))
  (bind _offsetp_2 (Variables|Default|GetOffsetP))
  (bind _returnvalue (Transformation|GetWorldTransform _rkp))
  (bind _returnvalue_2 (Transformation|GetWorldTransform _offsetp_2))
  (bind _returnvalue_3 (Transformation|GetWorldTransform _lkp))
  (bind _returnvalue_4 (Transformation|GetWorldTransform _offsetp))
  (bind _output_transform (CallFunction|MakeRelativeTransform _returnvalue _returnvalue_2))
  (bind _output_transform_2 (CallFunction|MakeRelativeTransform _returnvalue_3 _returnvalue_4))
  ;[1 1 1] Playback Recording
  (if PlaybackOffset
    (Transformation|SetWorldTransform (Variables|Default|GetVR%20Offset) (Transformation|GetWorldTransform (Variables|Default|GetOffsetP)) false false))
  (Transformation|SetRelativeTransform (Variables|Default|GetRightKnee) (Math|Transform|MakeTransform (.location _output_transform) (.rotation _output_transform) "0.100000,0.100000,0.100000") false false)
  (Transformation|SetRelativeTransform (Variables|Default|GetLeftKnee) (Math|Transform|MakeTransform (.location _output_transform_2) (.rotation _output_transform_2) "0.100000,0.100000,0.100000") false false)
  (Transformation|SetRelativeTransform (Variables|Default|GetVR%20Camera) (CallFunction|MakeRelativeTransform (Transformation|GetWorldTransform (Variables|Default|GetCamP)) (Transformation|GetWorldTransform (Variables|Default|GetOffsetP))) false false))

(event Custom|PlaybackSkateboard
  (bind _offsetp (Variables|Default|GetOffsetP))
  (bind _skatep (Variables|Default|GetSkateP))
  (bind _returnvalue (Transformation|GetWorldTransform _skatep))
  (bind _returnvalue_2 (Transformation|GetWorldTransform _offsetp))
  (bind _output_transform (CallFunction|MakeRelativeTransform _returnvalue _returnvalue_2))
  ;[1 1 1] Playback Skateboard
  (if (and (not (Utilities|IsValid (Variables|Default|GetSkateboard))) (Math|Vector|NotEqual(Vector) (Variables|/Script/Engine.SceneComponent|GetRelativeLocation (Variables|Default|GetSkateboardControl)) (.location (CallFunction|MakeRelativeTransform (Transformation|GetWorldTransform (Variables|Default|GetSkateP)) (Transformation|GetWorldTransform (Variables|Default|GetOffsetP)))) 1e+01))
    (CallFunction|SpawnSkateboard))
  (Transformation|SetRelativeTransform (Variables|Default|GetSkateboardControl) (Math|Transform|MakeTransform (.location _output_transform) (.rotation _output_transform) "1,1,1") false false))

(event Custom|Apply%20Goofy
  ;[1 1 1] Apply Goofy
  (if (Variables|Default|GetRegular)
    (if (not (> (Math|Vector|DotProduct (- (.OutPosition (Class|SteamVRFunctionLibrary|GetHandPositionandOrientation 0 "Left")) (.OutPosition (Class|SteamVRFunctionLibrary|GetHandPositionandOrientation 0 "Right"))) (Variables|Default|GetRealDirection)) 0.0))
      (Variables|Default|SetRealDirection (* (Variables|Default|GetRealDirection) -1.0) :!label _label)
      (Variables|Default|SetDirection (* (Variables|Default|GetDirection) -1.0)))
    (elif (> (Math|Vector|DotProduct (- (.OutPosition (Class|SteamVRFunctionLibrary|GetHandPositionandOrientation 0 "Left")) (.OutPosition (Class|SteamVRFunctionLibrary|GetHandPositionandOrientation 0 "Right"))) (Variables|Default|GetRealDirection)) 0.0)
      (goto _label))))

(event Custom|Spawn%20Skateboard
  (bind _vr_origin (Variables|Default|GetVR%20Origin))
  (bind _bodycenter (Variables|Default|GetBodyCenter))
  (bind _bodycenter_2 (Variables|Default|GetBodyCenter))
  (bind _rightknee (Variables|Default|GetRightKnee))
  (bind _returnvalue (Math|Vector|MakeVector (.x _bodycenter) (.y _bodycenter) 0.0))
  (bind _returnvalue_2 (Math|Vector|MakeVector (.x _bodycenter_2) (.y _bodycenter_2) 0.0))
  (bind _returnvalue_3 (Transformation|GetRelativeTransform _vr_origin))
  (bind _relativerotation (Variables|/Script/Engine.SceneComponent|GetRelativeRotation _rightknee))
  (bind _returnvalue_4 (Math|Rotator|MakeRotator 0.0 0.0 (.yaw _relativerotation)))
  (bind (_x _y) (Math|Vector|BreakVector _returnvalue_2))
  (bind _returnvalue_5 (* (.yaw (.rotation _returnvalue_3)) -1.0))
  ;[1 1 1] Spawn Skateboard
  (CallFunction|UpdateDirection)
  (bind _returnvalue_6 (Game|SpawnActorfromClass "/Game/Blueprints/Hoverboard.Hoverboard_C" (Math|Transform|MakeTransform "0, 0, 0" "0, 0, 0" "1,1,1.000000") "Undefined" 0 0))
  (bind _output_get (Variables|Default|SetSkateboard _returnvalue_6))
  (Transformation|AttachComponentToComponent _output_get (Variables|Default|GetSkateboardControl) "None" "KeepRelative" "KeepRelative" "KeepRelative" true)
  (Transformation|SetRelativeTransform (Variables|Default|GetSkateboardControl) (Math|Transform|MakeTransform (Math|Vector|RotateVectorAroundAxis (+ (* (Math|Vector|Normalize (Variables|Default|GetDirection)) -1e+03) (* (Math|Vector|RotateVectorAroundAxis (Math|Vector|Normalize (Variables|Default|GetDirection)) 9e+01 "0, 0,1.000000") 5e+01)) _returnvalue_5 "0, 0,1.000000") _returnvalue_4) false false)
  (if (< (Math|Vector|VectorLengthSquared _returnvalue) (Math|Float|Square 1e+02))
    (Variables|Default|SetSkateSpawn (+ _returnvalue (Math|Vector|MakeVector (* (Math|Float|Sign(Float) (.x _bodycenter)) (Variables|Default|GetBoardSpawnDist)) (* (Math|Float|Sign(Float) (.y _bodycenter)) (Variables|Default|GetBoardSpawnDist)) 0.0)))
    (bind _output_get_2 (Variables|Default|SetRotationThing (.rotation (Math|Transform|MakeTransform (Math|Vector|RotateVectorAroundAxis (+ (* (Math|Vector|RotateVectorAroundAxis (Math|Vector|Normalize (Variables|Default|GetDirection)) 9e+01 "0, 0,1.000000") 5e+01) (Math|Vector|MakeVector _x _y 0.0)) _returnvalue_5 "0, 0,1.000000") _returnvalue_4 "1.000000,1,1"))))
    (else
      (Variables|Default|SetSkateSpawn "0, 0,0.000000")))
  (Components|MoveComponentTo (Variables|Default|GetSkateboardControl) (Variables|Default|GetSkateSpawn) _output_get_2 true true 2.0 false)
  (Variables|Default|SetDirection (Math|Vector|GetForwardVector (Math|Rotator|CombineRotators _output_get_2 (Transformation|GetWorldRotation (Variables|Default|GetVR%20Offset)))))
  (Variables|Default|SetRealDirection (Math|Vector|GetForwardVector _output_get_2)))

(event Custom|UpdateKnee
  (bind (_outposition _outorientation) (Class|SteamVRFunctionLibrary|GetHandPositionandOrientation 0 "Left"))
  (bind (_outposition_2 _outorientation_2) (Class|SteamVRFunctionLibrary|GetHandPositionandOrientation 0 "Right"))
  ;[1 1 1] Update Knee Transform
  (Transformation|SetRelativeTransform (Variables|Default|GetRightKnee) (Math|Transform|MakeTransform _outposition_2 (Math|Rotator|CombineRotators "0,90.000000, 0" (Class|QuaternionFunctions|ConverttoRotator (Class|QuaternionFunctions|CombineQuaternions (Class|QuaternionFunctions|ConverttoQuaternion _outorientation_2) (Utilities|Struct|MakeQuat (Variables|Default|GetInitialRotationX) (Variables|Default|GetInitialRotationY) (Variables|Default|GetInitialRotationZ) (Variables|Default|GetInitialRotationW))))) "0.100000,0.100000,0.100000") false false)
  (Transformation|SetRelativeTransform (Variables|Default|GetLeftKnee) (Math|Transform|MakeTransform _outposition (Math|Rotator|CombineRotators "0,90.000000, 0" (Class|QuaternionFunctions|ConverttoRotator (Class|QuaternionFunctions|CombineQuaternions (Class|QuaternionFunctions|ConverttoQuaternion _outorientation) (Utilities|Struct|MakeQuat (Variables|Default|GetRightRotationX) (Variables|Default|GetRightRotationY) (Variables|Default|GetRightRotationZ) (Variables|Default|GetRightRotationW))))) "0.100000,0.100000,0.100000") false false))

(event EventBeginPlay
  (bind (_outposition _outorientation) (Class|SteamVRFunctionLibrary|GetHandPositionandOrientation 0 "Right"))
  (bind _outorientation_2 (Class|SteamVRFunctionLibrary|GetHandPositionandOrientation 0 "Left"))
  (bind (_outposition_2 _outorientation_3) (Class|SteamVRFunctionLibrary|GetHandPositionandOrientation 0 "Right"))
  (bind _skateboard (Variables|Default|GetSkateboard))
  (bind _returnvalue (Class|QuaternionFunctions|ConverttoQuaternion _outorientation))
  (bind _returnvalue_2 (Class|QuaternionFunctions|ConverttoQuaternion _outorientation_2))
  (bind _returnvalue_3 (Class|QuaternionFunctions|InvertQuaternion _returnvalue_2))
  (bind _returnvalue_4 (Class|QuaternionFunctions|InvertQuaternion _returnvalue))
  ;[1 1 1] Initial Values
  (Utilities|FlowControl|Delay 1.0)
  (bind _output_get (Variables|Default|SetKneeHeight (.z _outposition)))
  (Transformation|SetRelativeLocation (Variables|Default|GetRightFoot) (Math|Vector|MakeVector 0.0 0.0 (* _output_get -1e+01)) false false)
  (Variables|Default|SetHeightOffset (- (.z (Transformation|GetWorldLocation (Variables|Default|GetRightKnee))) (Variables|Default|GetKneeHeight)))
  (Transformation|SetRelativeLocation (Variables|Default|GetLeftFoot) (Math|Vector|MakeVector 0.0 0.0 (* _output_get -1e+01)) false false)
  (Variables|Default|SetInitialRightVector (- (.OutPosition (Class|SteamVRFunctionLibrary|GetHandPositionandOrientation 0 "Left")) _outposition_2))
  (Variables|Default|SetInitialRightPitch (.yaw _outorientation_3))
  (Variables|Default|SetInitialRotation _outorientation)
  (Variables|Default|SetInitialRotationX (.x _returnvalue_4))
  (Variables|Default|SetInitialRotationY (.y _returnvalue_4))
  (Variables|Default|SetInitialRotationZ (.z _returnvalue_4))
  (Variables|Default|SetInitialRotationW (.w _returnvalue_4))
  (Variables|Default|SetRightRotationX (.x _returnvalue_3))
  (Variables|Default|SetRightRotationY (.y _returnvalue_3))
  (Variables|Default|SetRightRotationZ (.z _returnvalue_3))
  (Variables|Default|SetRightRotationW (.w _returnvalue_3))
  (if (Utilities|IsValid _skateboard)
    (Actor|DestroyActor _skateboard)))

(event Collision|EventActorBeginOverlap
  (params (OtherActor :type Actor%20Object%20Reference)))

(event EventTick
  (params (DeltaSeconds :type Float%20%28single-precision%29))
  (bind _box (Variables|Default|GetBox))
  (bind _box_2 (Variables|Default|GetBox))
  (if (Variables|Default|GetPlayback)
    (CallFunction|PlaybackData true)
    (CallFunction|PlaybackSkateboard)
    (Utilities|FlowControl|Sequence :!label _label
      (:then_0
        ;[1 1 1] Update Body Center
        (Variables|Default|SetBodyCenter (/ (+ (Variables|/Script/Engine.SceneComponent|GetRelativeLocation (Variables|Default|GetRightKnee)) (Variables|/Script/Engine.SceneComponent|GetRelativeLocation (Variables|Default|GetLeftKnee))) 2.0)))
      (:then_1
        ;[1 1 1] Update Lean
        (Variables|Default|SetLean (+ (* (Math|Vector|RotateVectorAroundAxis (- (Variables|/Script/Engine.SceneComponent|GetRelativeLocation (Variables|Default|GetVR%20Camera)) (Variables|Default|GetBodyCenter)) (* (.yaw (Math|Rotator|MakeRotfromX (Variables|Default|GetRealDirection))) -1.0) "0, 0,1.000000") "1.000000,1.000000, 0") "0.000000, 0, 0")))
      (:then_2
        ;[1 1 1] Check if skating
        (if (Variables|Default|GetSkating)
          ;[1 1 1] Rotate Skateboard
          (Variables|Default|SetDirection (Math|Vector|RotateVectorAroundAxis (Variables|Default|GetDirection) (* (* (Class|TransformationFunctions|ApplyThreshold (Math|Float|Clamp(Float) (/ (.y (Variables|Default|GetLean)) (Variables|Default|GetLeanClamp)) -1.0) (Variables|Default|GetLeanThreshold)) (Variables|Default|GetTurnSpeed)) DeltaSeconds) "0, 0,1.000000"))
          (Class|TransformationFunctions|AddWorldRotationAroundPivot (Variables|Default|GetVR%20Origin) (Transformation|GetWorldLocation (Variables|Default|GetVR%20Camera)) (* (Math|Vector|MakeVector 0.0 0.0 1.0) (* (* (Class|TransformationFunctions|ApplyThreshold (Math|Float|Clamp(Float) (/ (.y (Variables|Default|GetLean)) (Variables|Default|GetLeanClamp)) -1.0) (Variables|Default|GetLeanThreshold)) (Variables|Default|GetTurnSpeed)) DeltaSeconds)))
          ;[1 1 1] Accelerate Skateboard
          (if (== (Math|Float|Sign(Float) (.x (Variables|Default|GetLean))) 1.0)
            (Variables|Default|SetSkateSpeed (Math|Float|Clamp(Float) (+ (* (* (Class|TransformationFunctions|ApplyThreshold (Math|Float|Clamp(Float) (/ (.x (Variables|Default|GetLean)) (Variables|Default|GetLeanClamp)) -1.0) (Variables|Default|GetLeanThreshold)) (* (Variables|Default|GetAcceleration) DeltaSeconds)) (/ (- (Variables|Default|GetMaxSpeed) (Variables|Default|GetSkateSpeed)) (Variables|Default|GetMaxSpeed))) (Variables|Default|GetSkateSpeed)) 0.0 (Variables|Default|GetMaxSpeed)))
            (else
              (Variables|Default|SetSkateSpeed (Math|Float|Clamp(Float) (+ (* (Class|TransformationFunctions|ApplyThreshold (Math|Float|Clamp(Float) (/ (.x (Variables|Default|GetLean)) (Variables|Default|GetLeanClamp)) -1.0) (Variables|Default|GetLeanThreshold)) (* (Variables|Default|GetBrakingSpeed) DeltaSeconds)) (Variables|Default|GetSkateSpeed)) 0.0 (Variables|Default|GetMaxSpeed)))))
          ;[1 1 1] Translate Skateboard
          (Transformation|AddWorldOffset (Variables|Default|GetVR%20Origin) (* (* (Variables|Default|GetDirection) (Variables|Default|GetSkateSpeed)) DeltaSeconds) false false)
          ;[1 1 1] Check if user has stepped off
          (if (and (not (Class|PrimitiveComponent|IsOverlappingComponent (Variables|Default|GetRightFoot) _box_2)) (not (Class|PrimitiveComponent|IsOverlappingComponent (Variables|Default|GetLeftFoot) _box_2)))
            (CallFunction|StopSkate))
          (else
            ;[1 1 1] Check if on top of skateboard
            (if (Utilities|IsValid (Variables|Default|GetSkateboard))
              (if (and (Class|PrimitiveComponent|IsOverlappingComponent (Variables|Default|GetRightFoot) _box) (Class|PrimitiveComponent|IsOverlappingComponent (Variables|Default|GetLeftFoot) _box))
                (Utilities|FlowControl|Delay 1.0)
                (CallFunction|StartSkate)))))))
    (elif (and (.ReturnValue (Class|SteamVRFunctionLibrary|GetHandPositionandOrientation 0 "Right")) (.ReturnValue (Class|SteamVRFunctionLibrary|GetHandPositionandOrientation 0 "Left")))
      (CallFunction|UpdateKnee)
      (goto _label)
      (else
        (Development|PrintString "ERROR ERROR ERROR" true true "(R=1.000000,G=0.007701,B=0.000000,A=1.000000)")))))

(event Input|ActionEvents|InputActionCalibrate
  (params (Key :type Key%20Structure :default "AnyKey"))
  (bind (_outposition _outorientation) (Class|SteamVRFunctionLibrary|GetHandPositionandOrientation 0 "Right"))
  (bind _outorientation_2 (Class|SteamVRFunctionLibrary|GetHandPositionandOrientation 0 "Left"))
  (bind (_outposition_2 _outorientation_3) (Class|SteamVRFunctionLibrary|GetHandPositionandOrientation 0 "Right"))
  (bind _skateboard (Variables|Default|GetSkateboard))
  (bind _returnvalue (Class|QuaternionFunctions|ConverttoQuaternion _outorientation))
  (bind _returnvalue_2 (Class|QuaternionFunctions|ConverttoQuaternion _outorientation_2))
  (bind _returnvalue_3 (Class|QuaternionFunctions|InvertQuaternion _returnvalue_2))
  (bind _returnvalue_4 (Class|QuaternionFunctions|InvertQuaternion _returnvalue))
  ;[1 1 1] Initial Values
  (:Pressed
    (Utilities|FlowControl|Delay 1.0)
    (bind _output_get (Variables|Default|SetKneeHeight (.z _outposition)))
    (Transformation|SetRelativeLocation (Variables|Default|GetRightFoot) (Math|Vector|MakeVector 0.0 0.0 (* _output_get -1e+01)) false false)
    (Variables|Default|SetHeightOffset (- (.z (Transformation|GetWorldLocation (Variables|Default|GetRightKnee))) (Variables|Default|GetKneeHeight)))
    (Transformation|SetRelativeLocation (Variables|Default|GetLeftFoot) (Math|Vector|MakeVector 0.0 0.0 (* _output_get -1e+01)) false false)
    (Variables|Default|SetInitialRightVector (- (.OutPosition (Class|SteamVRFunctionLibrary|GetHandPositionandOrientation 0 "Left")) _outposition_2))
    (Variables|Default|SetInitialRightPitch (.yaw _outorientation_3))
    (Variables|Default|SetInitialRotation _outorientation)
    (Variables|Default|SetInitialRotationX (.x _returnvalue_4))
    (Variables|Default|SetInitialRotationY (.y _returnvalue_4))
    (Variables|Default|SetInitialRotationZ (.z _returnvalue_4))
    (Variables|Default|SetInitialRotationW (.w _returnvalue_4))
    (Variables|Default|SetRightRotationX (.x _returnvalue_3))
    (Variables|Default|SetRightRotationY (.y _returnvalue_3))
    (Variables|Default|SetRightRotationZ (.z _returnvalue_3))
    (Variables|Default|SetRightRotationW (.w _returnvalue_3))
    (if (Utilities|IsValid _skateboard)
      (Actor|DestroyActor _skateboard))))

(event Input|KeyboardEvents|Up
  (params (Key :type Key%20Structure :default "AnyKey"))
  (:Pressed
    (Variables|Default|SetNewVar_0 (+ (Variables|Default|GetNewVar_0) 5.0))))

(event Input|KeyboardEvents|Down
  (params (Key :type Key%20Structure :default "AnyKey"))
  (:Pressed
    (Variables|Default|SetNewVar_0 (+ (Variables|Default|GetNewVar_0) -5.0))))

(event Input|KeyboardEvents|Left
  (params (Key :type Key%20Structure :default "AnyKey"))
  (:Pressed
    (Variables|Default|SetNewVar_1 (+ (Variables|Default|GetNewVar_1) 5.0))))

(event Input|KeyboardEvents|Right
  (params (Key :type Key%20Structure :default "AnyKey"))
  (:Pressed
    (Variables|Default|SetNewVar_1 (+ (Variables|Default|GetNewVar_1) -5.0))))

(event Input|KeyboardEvents|B
  (params (Key :type Key%20Structure :default "AnyKey"))
  (:Pressed
    (Variables|Default|SetNewVar_2 (+ (Variables|Default|GetNewVar_2) 5.0))))

(event Input|KeyboardEvents|N
  (params (Key :type Key%20Structure :default "AnyKey"))
  (:Pressed
    (Variables|Default|SetNewVar_2 (+ (Variables|Default|GetNewVar_2) -5.0))))

(event Input|KeyboardEvents|SpaceBar
  (params (Key :type Key%20Structure :default "AnyKey"))
  (bind _vr_origin (Variables|Default|GetVR%20Origin))
  (bind _bodycenter (Variables|Default|GetBodyCenter))
  (bind _bodycenter_2 (Variables|Default|GetBodyCenter))
  (bind _rightknee (Variables|Default|GetRightKnee))
  (bind _returnvalue (Math|Vector|MakeVector (.x _bodycenter) (.y _bodycenter) 0.0))
  (bind _returnvalue_2 (Math|Vector|MakeVector (.x _bodycenter_2) (.y _bodycenter_2) 0.0))
  (bind _returnvalue_3 (Transformation|GetRelativeTransform _vr_origin))
  (bind _relativerotation (Variables|/Script/Engine.SceneComponent|GetRelativeRotation _rightknee))
  (bind _returnvalue_4 (Math|Rotator|MakeRotator 0.0 0.0 (.yaw _relativerotation)))
  (bind (_x _y) (Math|Vector|BreakVector _returnvalue_2))
  (bind _returnvalue_5 (* (.yaw (.rotation _returnvalue_3)) -1.0))
  ;[1 1 1] Spawn Skateboard
  (:Pressed
    (if (not (Variables|Default|GetPlayback))
      (if (not (Variables|Default|GetSkating))
        (CallFunction|UpdateDirection)
        (bind _returnvalue_6 (Game|SpawnActorfromClass "/Game/Blueprints/Hoverboard.Hoverboard_C" (Math|Transform|MakeTransform "0, 0, 0" "0, 0, 0" "1,1,1.000000") "Undefined" 0 0))
        (bind _output_get (Variables|Default|SetSkateboard _returnvalue_6))
        (Transformation|AttachComponentToComponent _output_get (Variables|Default|GetSkateboardControl) "None" "KeepRelative" "KeepRelative" "KeepRelative" true)
        (Transformation|SetRelativeTransform (Variables|Default|GetSkateboardControl) (Math|Transform|MakeTransform (Math|Vector|RotateVectorAroundAxis (+ (* (Math|Vector|Normalize (Variables|Default|GetDirection)) -1e+03) (* (Math|Vector|RotateVectorAroundAxis (Math|Vector|Normalize (Variables|Default|GetDirection)) 9e+01 "0, 0,1.000000") 5e+01)) _returnvalue_5 "0, 0,1.000000") _returnvalue_4) false false)
        (if (< (Math|Vector|VectorLengthSquared _returnvalue) (Math|Float|Square 1e+02))
          (Variables|Default|SetSkateSpawn (+ _returnvalue (Math|Vector|MakeVector (* (Math|Float|Sign(Float) (.x _bodycenter)) (Variables|Default|GetBoardSpawnDist)) (* (Math|Float|Sign(Float) (.y _bodycenter)) (Variables|Default|GetBoardSpawnDist)) 0.0)))
          (bind _output_get_2 (Variables|Default|SetRotationThing (.rotation (Math|Transform|MakeTransform (Math|Vector|RotateVectorAroundAxis (+ (* (Math|Vector|RotateVectorAroundAxis (Math|Vector|Normalize (Variables|Default|GetDirection)) 9e+01 "0, 0,1.000000") 5e+01) (Math|Vector|MakeVector _x _y 0.0)) _returnvalue_5 "0, 0,1.000000") _returnvalue_4 "1.000000,1,1"))))
          (else
            (Variables|Default|SetSkateSpawn "0, 0,0.000000")))
        (Components|MoveComponentTo (Variables|Default|GetSkateboardControl) (Variables|Default|GetSkateSpawn) _output_get_2 true true 2.0 false)
        (Variables|Default|SetDirection (Math|Vector|GetForwardVector (Math|Rotator|CombineRotators _output_get_2 (Transformation|GetWorldRotation (Variables|Default|GetVR%20Offset)))))
        (Variables|Default|SetRealDirection (Math|Vector|GetForwardVector _output_get_2))))))

(fn ConstructionScript)

(fn IsGrounded
  (params (Threshold :type Float%20%28single-precision%29))
  (return (< (.z (Transformation|GetWorldLocation (Variables|Default|GetRightFoot))) Threshold) (< (.z (Transformation|GetWorldLocation (Variables|Default|GetLeftFoot))) Threshold)))

(fn MakeRelativeTransform
  (params (Input%20Transform :type Transform) (Parent%20Transform :type Transform))
  (return (Math|Transform|MakeTransform (- (.location Input%20Transform) (.location Parent%20Transform)) (Math|Rotator|CombineRotators (.rotation Input%20Transform) (Class|KismetMathLibrary|NegateRotator (.rotation Parent%20Transform))) (* (.scale Input%20Transform) (.scale Parent%20Transform)))))