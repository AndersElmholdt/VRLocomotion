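; Hoverboard actor that banks its mesh into turns and can be destroyed with an effect.
; Tick derives roll from the yaw change since last frame, smoothing and clamping it on the static mesh.
; Kill spawns a particle emitter, then after short delays removes the mesh, particle and light components before destroying the actor.
; IsAlive reads inverted: Kill sets it true, which stops the tilt update.
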(event Custom|Kill
  (bind _returnvalue (Transformation|GetActorTransform))
  (Effects|SpawnEmitteratLocation "/Game/NewParticleSystem.NewParticleSystem" (.location _returnvalue) (.rotation _returnvalue))
  (Utilities|FlowControl|Delay 0.3)
  (Variables|Default|SetIsAlive true)
  (Components|DestroyComponent (Variables|Default|GetStaticMesh))
  (Components|DestroyComponent (Variables|Default|GetParticleSystem))
  (Components|DestroyComponent (Variables|Default|GetPointLight))
  (Utilities|FlowControl|Delay 0.7)
  (Actor|DestroyActor))

(event EventBeginPlay)

(event Collision|EventActorBeginOverlap
  (params (OtherActor :type Actor%20Object%20Reference)))

(event EventTick
  (params (DeltaSeconds :type Float%20%28single-precision%29))
  (bind _staticmesh (Variables|Default|GetStaticMesh))
  (if (not (Variables|Default|GetIsAlive))
    (Utilities|FlowControl|Sequence
      (:then_0
        (Transformation|SetRelativeRotation _staticmesh (Math|Rotator|MakeRotator (Math|Float|Clamp(Float) (Math|Float|Lerp (.roll (Variables|/Script/Engine.SceneComponent|GetRelativeRotation _staticmesh)) (* (.yaw (Math|Rotator|Delta(Rotator) (Transformation|GetActorRotation) (Variables|Default|GetPreviousOrientation))) (* (Variables|Default|GetTiltScale) DeltaSeconds)) 0.2) -45.0 45.0) 0.0 0.0) false false))
      (:then_1
        (Variables|Default|SetPreviousLocation (Transformation|GetActorLocation))
        (Variables|Default|SetPreviousOrientation (Transformation|GetActorRotation))))))

(fn ConstructionScript)