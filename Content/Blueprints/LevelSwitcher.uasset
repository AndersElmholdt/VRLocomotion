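; LevelSwitcher is an actor that moves the player to another level when they are overlapping and facing the required direction.
; StartOverlap and EndOverlap set a flag that Tick checks before comparing the Virtuotion pawn's VR camera yaw to the actor's yaw within a tolerance.
; A match plays the FadeOut level sequence once, and its stop event opens NewLevel.
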(event Custom|ChangeLevel
  (Game|OpenLevel(byName) (Variables|Default|GetNewLevel)))

(event EventBeginPlay)

(event Collision|EventActorBeginOverlap
  (params (OtherActor :type Actor%20Object%20Reference)))

(event EventEndOverlap
  (Variables|Default|SetIsOverlapping false))

(event EventTick
  (params (DeltaSeconds :type Float%20%28single-precision%29))
  (if (Variables|Default|GetIsOverlapping)
    (bind _asvirtuotion (Utilities|Casting|CastToVirtuotion (Game|Player|GetPlayerPawn 0)))
    (if (Math|Float|NearlyEqual(Float) (.yaw (Transformation|GetWorldRotation (Variables|/Game/Blueprints/Virtuotion.Virtuotion_C|GetVR%20Camera _asvirtuotion))) (.yaw (Transformation|GetActorRotation)) 1e+01)
      (Utilities|FlowControl|DoOnce false
        (:Completed
          (bind _returnvalue (Sequencer|Player|CreateLevelSequencePlayer "/Game/FadeOut.FadeOut"))
          (EventDispatchers|BindEventtoOnStop _returnvalue (delegate Custom|ChangeLevel))
          (Sequencer|Player|Play _returnvalue :!class /Script/MovieScene.MovieSceneSequencePlayer))))))

(event EventStartOverlap
  (Variables|Default|SetIsOverlapping true))

(fn ConstructionScript)