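; PathFollower is an actor that mirrors the world transform of a component attached to the Usability_Pawn's camera.
; While Loop is true, Tick searches all Usability_Pawn actors, stores the camera's first direct child as FollowObject and clears Loop.
; Once Loop is false, each Tick copies FollowObject's world location and rotation onto DefaultSceneRoot, without sweep.
; The SearchForActor event is an empty stub.
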(event Custom|SearchForActor)

(event EventBeginPlay)

(event Collision|EventActorBeginOverlap
  (params (OtherActor :type Actor%20Object%20Reference)))

(event EventTick
  (params (DeltaSeconds :type Float%20%28single-precision%29))
  (if (Variables|Default|GetLoop)
    (bind _outactors (Actor|GetAllActorsOfClass "/Game/Blueprints/Usability_Pawn.Usability_Pawn_C"))
    (for _array_element _outactors
      (for (_array_element_2 _array_index) (Components|GetChildrenComponents (Variables|/Game/Blueprints/Usability_Pawn.Usability_Pawn_C|GetCamera _array_element) false)
        (if (== _array_index 0)
          (Variables|Default|SetFollowObject _array_element_2)
          (Variables|Default|SetLoop false))))
    (else
      (Transformation|SetWorldLocation (Variables|Default|GetDefaultSceneRoot) (Transformation|GetWorldLocation (Variables|Default|GetFollowObject)) false false)
      (Transformation|SetWorldRotation (Variables|Default|GetDefaultSceneRoot) (Transformation|GetWorldRotation (Variables|Default|GetFollowObject)) false false))))

(fn ConstructionScript)