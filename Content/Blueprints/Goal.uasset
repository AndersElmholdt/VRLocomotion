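; Goal actor that consumes balls entering it and signals a win when the last one is in.
; Tick spins StaticMesh1 around yaw at a steady, frame-rate independent speed.
; Capsule overlap destroys any Ball actor and decrements AmountOfBalls, then at zero prints a burst of randomly colored congratulation messages via PrintString.
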(event OnComponentBeginOverlap(Capsule)
  (params (OverlappedComponent :type Primitive%20Component%20Object%20Reference) (OtherActor :type Actor%20Object%20Reference) (OtherComp :type Primitive%20Component%20Object%20Reference) (OtherBodyIndex :type Integer) (bFromSweep :type Boolean) (SweepResult :type Hit%20Result%20Structure%20%28by%20ref%29))
  (bind _returnvalue (Math|Random|RandomFloat))
  (bind _asball (Utilities|Casting|CastToBall OtherActor))
  (Actor|DestroyActor _asball)
  (bind _output_get (Variables|Default|SetAmountOfBalls (- (Variables|Default|GetAmountOfBalls) 1)))
  (if (== _output_get 0)
    (for _index (range 0 100)
      (Development|PrintString "CONGRATULATIONS!!!!!" true true (Math|Color|MakeColor _returnvalue _returnvalue _returnvalue)))))

(event EventBeginPlay)

(event Collision|EventActorBeginOverlap
  (params (OtherActor :type Actor%20Object%20Reference)))

(event EventTick
  (params (DeltaSeconds :type Float%20%28single-precision%29))
  (bind _staticmesh1 (Variables|Default|GetStaticMesh1))
  (Transformation|SetRelativeRotation _staticmesh1 (Math|Rotator|CombineRotators (Variables|/Script/Engine.SceneComponent|GetRelativeRotation _staticmesh1) (Math|Rotator|MakeRotator 0.0 0.0 (* DeltaSeconds 45.0))) false false))

(fn ConstructionScript)